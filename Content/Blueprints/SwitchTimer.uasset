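; SwitchTimer is a Blueprint countdown timer that tracks one named channel at a time, with settings looked up from TimerTable.
; DelayTimeCheck subtracts world delta time on each call and returns true once the time runs out.
; Requesting a different channel loads its entry and restarts the countdown, or prints an error if none exists.
; Entries flagged EndReset restart on expiry, carrying the overshoot into the next cycle.
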(fn DelayTimeCheck
  (params (Channel :type Integer))
  (bind _timertable (Variables|Default|GetTimerTable))
  (bind (_value _returnvalue) (Utilities|Map|Find _timertable Channel))
  (if (== Channel (Variables|Default|GetCurrentChannel))
    (bind _output_get (Variables|Default|SetTimer (- (Variables|Default|GetTimer) (Utilities|Time|GetWorldDeltaSeconds)) :!label _label))
    (if (<= _output_get 0.0)
      (if (.EndReset (Utilities|Struct|BreakTimerBase (Variables|Default|GetCurrentTimer)))
        (Variables|Default|SetTimer (+ (.Time (Utilities|Struct|BreakTimerBase (Variables|Default|GetCurrentTimer))) (Variables|Default|GetTimer))))
      (return true)
      (else
        (return false)))
    (elif _returnvalue
      (Variables|Default|SetCurrentChannel Channel)
      (bind _output_get_2 (Variables|Default|SetCurrentTimer _value))
      (Variables|Default|SetTimer (.Time (Utilities|Struct|BreakTimerBase _output_get_2)))
      (goto _label)
      (else
        (Development|PrintText "Channel Not Exists")))))