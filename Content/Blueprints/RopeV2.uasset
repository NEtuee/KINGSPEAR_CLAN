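; RopeV2 is a swingable rope actor that the player can grab, climb and optionally destroy.
; Its Box overlap flags the player as able to grab and passes it a rope reference.
; Climb input changes the clamped length, repositioning RopeMiddle along the rope's direction, rebinding its constraint to RopeStart, and resizing the Box and both cables.
; Swinging applies force to RopeMiddle as an acceleration change.
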(event OnComponentBeginOverlap(Box)
  (params (OverlappedComponent :type Primitive%20Component%20Object%20Reference) (OtherActor :type Actor%20Object%20Reference) (OtherComp :type Primitive%20Component%20Object%20Reference) (OtherBodyIndex :type Integer) (bFromSweep :type Boolean) (SweepResult :type Hit%20Result%20Structure%20%28by%20ref%29))
  (Development|PrintText "Hello")
  (bind _value (Class|BPIPlayer|IsPlayer(Message) OtherActor))
  (if _value
    (bind _asihateunreal (Utilities|Casting|CastToIHATEUNREAL OtherActor))
    (Variables|/Game/Blueprints/IHATEUNREAL.IHATEUNREAL_C|SetCanGrabRope _asihateunreal true)
    (Variables|/Game/Blueprints/IHATEUNREAL.IHATEUNREAL_C|SetRopeV2 _asihateunreal self)))

(event OnComponentEndOverlap(Box)
  (params (OverlappedComponent :type Primitive%20Component%20Object%20Reference) (OtherActor :type Actor%20Object%20Reference) (OtherComp :type Primitive%20Component%20Object%20Reference) (OtherBodyIndex :type Integer))
  (bind _value (Class|BPIPlayer|IsPlayer(Message) OtherActor))
  (if _value
    (bind _asihateunreal (Utilities|Casting|CastToIHATEUNREAL OtherActor))
    (Variables|/Game/Blueprints/IHATEUNREAL.IHATEUNREAL_C|SetCanGrabRope _asihateunreal false)))

(event Custom|DestroyRope
  (if (Variables|Default|GetIsDestroyable)
    (Actor|DestroyActor)))

(event Custom|AddSwingForce
  (params (Force :type Vector) (Multiple :type Float%20%28single-precision%29))
  (Physics|AddForce (Variables|Default|GetRopeMiddle) (* Force Multiple) "None" true))

(event Custom|UpdateRope
  (params (TargetLength :type Float%20%28single-precision%29) (UpdateBox :type Boolean))
  (bind _box (Variables|Default|GetBox))
  (bind _ropestart (Variables|Default|GetRopeStart))
  (bind _returnvalue (Transformation|GetWorldLocation _ropestart))
  (bind _boxextent (Variables|/Script/Engine.BoxComponent|GetBoxExtent _box))
  (if (>= TargetLength (Variables|Default|GetCableLength))
    (Variables|Default|SetCurrentCableLength (Variables|Default|GetCableLength))
    (else
      (Variables|Default|SetCurrentCableLength TargetLength)))
  (Transformation|SetWorldLocation (Variables|Default|GetRopeMiddle) (+ (* (Math|Vector|Normalize (- (Transformation|GetWorldLocation (Variables|Default|GetRopeMiddle)) _returnvalue)) (Variables|Default|GetCurrentCableLength)) _returnvalue) false true)
  (Class|PhysicsConstraintComponent|SetConstrainedComponents (Variables|Default|GetMiddleConstraint) (Variables|Default|GetRopeStart) "None" (Variables|Default|GetRopeMiddle) "None")
  (Transformation|SetRelativeLocation (Variables|Default|GetBox) (Math|Vector|MakeVector 0.0 0.0 (* (Variables|Default|GetCurrentCableLength) 0.5)) false true)
  (Components|Box|SetBoxExtent (Variables|Default|GetBox) (Math|Vector|MakeVector (.x _boxextent) (.y _boxextent) (* (Variables|Default|GetCurrentCableLength) 0.5)) true)
  (Variables|/Script/CableComponent.CableComponent|SetCableLength (Variables|Default|GetEndCable) (- (Variables|Default|GetCableLength) (Variables|Default|GetCurrentCableLength)))
  (Variables|/Script/CableComponent.CableComponent|SetCableLength (Variables|Default|GetMiddleCable) (* (Variables|Default|GetCurrentCableLength) 0.7)))

(event Custom|GoUpDown
  (params (Direction :type Float%20%28single-precision%29) (Speed :type Float%20%28single-precision%29) (Reverse :type Float%20%28single-precision%29))
  (bind _out (CallFunction|CableLengthLimitter (+ (Variables|Default|GetCurrentCableLength) (* (* (* Direction Reverse) Speed) (Utilities|Time|GetWorldDeltaSeconds)))))
  (CallFunction|UpdateRope _out false))

(event EventBeginPlay
  (CallFunction|UpdateRope (Variables|Default|GetCableLength) false))

(fn ConstructionScript)

(fn CableLengthLimitter
  (params (length :type Float%20%28single-precision%29))
  (bind _cablelength (Variables|Default|GetCableLength))
  (bind _lengthlimit (Variables|Default|GetLengthLimit))
  (if (>= length _cablelength)
    (return _cablelength)
    (elif (<= length _lengthlimit)
      (return _lengthlimit)
      (else
        (return length)))))