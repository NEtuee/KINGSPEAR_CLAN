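; Rope is a swingable rope actor that a player can grab.
; When its Collision component overlaps an actor that reports itself as the player, it sends that actor a GrabRope message with itself as reference.
; AddSwingForce applies a scaled force as an acceleration change to the CableEnd component.
; DestroyRope destroys the actor only when IsDestroyable is set.
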(event OnComponentBeginOverlap(Collision)
  (params (OverlappedComponent :type Primitive%20Component%20Object%20Reference) (OtherActor :type Actor%20Object%20Reference) (OtherComp :type Primitive%20Component%20Object%20Reference) (OtherBodyIndex :type Integer) (bFromSweep :type Boolean) (SweepResult :type Hit%20Result%20Structure%20%28by%20ref%29))
  (bind _value (Class|BPIPlayer|IsPlayer(Message) OtherActor))
  (if _value
    (Class|BPIPlayer|GrabRope(Message) OtherActor self)))

(event Custom|DestroyRope
  (if (Variables|Default|GetIsDestroyable)
    (Actor|DestroyActor)))

(event Custom|AddSwingForce
  (params (Force :type Vector))
  (Physics|AddForce (Variables|Default|GetCableEnd) (* Force 5e+02) "None" true))

(event EventBeginPlay)

(event Collision|EventActorBeginOverlap
  (params (OtherActor :type Actor%20Object%20Reference)))

(event EventTick
  (params (DeltaSeconds :type Float%20%28single-precision%29)))

(fn ConstructionScript)