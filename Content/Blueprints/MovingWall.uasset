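; MovingWall is a wall Blueprint whose Cube component oscillates back and forth around its starting position.
; BeginPlay caches the Cube's world location as the center of motion.
; Each Tick advances an angle by Speed and offsets the Cube along MoveDirection by its degree-based cosine, scaled by MoveDistance.
; The move teleports without sweeping, so collisions along the path do not block it.
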(event EventBeginPlay
  (Variables|Default|SetBeginLocation (Transformation|GetWorldLocation (Variables|Default|GetCube))))

(event EventTick
  (params (DeltaSeconds :type Float%20%28single-precision%29))
  (bind _output_get (Variables|Default|Setangle (+ (* DeltaSeconds (Variables|Default|Getspeed)) (Variables|Default|Getangle))))
  (Transformation|SetWorldLocation (Variables|Default|GetCube) (+ (* (* (Variables|Default|GetMoveDirection) (Math|Trig|Cos(Degrees) _output_get)) (Variables|Default|GetMoveDistance)) (Variables|Default|GetBeginLocation)) false true))

(fn ConstructionScript)