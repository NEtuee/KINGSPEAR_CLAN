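; Thrown spear projectile that sticks into what it hits and can be picked back up by the player.
; On hitting anything that is not a player, it zeroes projectile velocity and gravity, flags itself stopped and attaches its box to the hit component, keeping world transform.
; When a player overlaps the stopped spear, it sends a grab message and destroys itself, using interface calls to identify and notify the player.
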(event EventBeginPlay)

(event EventTick
  (params (DeltaSeconds :type Float%20%28single-precision%29)))

(event Collision|EventHit
  (params (MyComp :type Primitive%20Component%20Object%20Reference) (Other :type Actor%20Object%20Reference) (OtherComp :type Primitive%20Component%20Object%20Reference) (bSelfMoved :type Boolean) (HitLocation :type Vector :default "0, 0, 0") (HitNormal :type Vector :default "0, 0, 0") (NormalImpulse :type Vector :default "0, 0, 0") (Hit :type Hit%20Result%20Structure%20%28by%20ref%29))
  (bind _projectile (Variables|Default|GetProjectile))
  (bind _value (Class|BPIPlayer|IsPlayer(Message) Other))
  (if (not _value)
    (Development|PrintText "Collision")
    (Variables|/Script/Engine.MovementComponent|SetVelocity _projectile "0, 0, 0")
    (Variables|/Script/Engine.ProjectileMovementComponent|SetProjectileGravityScale _projectile 0.0)
    (Variables|Default|SetIsStop true)
    (Transformation|AttachComponentToComponent (Variables|Default|GetBox) OtherComp "None" "KeepWorld" "KeepWorld" "KeepWorld" true)))

(event Collision|EventActorBeginOverlap
  (params (OtherActor :type Actor%20Object%20Reference))
  (bind _value (Class|BPIPlayer|IsPlayer(Message) OtherActor))
  (if _value
    (if (Variables|Default|GetIsStop)
      (Class|BPIPlayer|GrabSpear(Message) OtherActor)
      (Actor|DestroyActor))))

(fn ConstructionScript)